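; Zombie enemy that chases the player on sight, attacks in melee and ragdolls when its health runs out.
; Pawn sensing triggers an AI move toward player 0, and reaching the target starts the attack.
; Each attack plays a montage and immediately applies damage, with a DoOnce reset after a delay as cooldown.
; Incoming damage lowers Health; at zero the mesh simulates physics, with no logic here stopping the AI.
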(event OnSeePawn(PawnSensing)
  (params (Pawn :type Pawn%20Object%20Reference))
  (Variables|Default|SetIsSeeingPlayer? true)
  (CallFunction|FollowPlayer))

(event Custom|FollowPlayer
  (Variables|Default|SetCanAttack? true)
  (if (Variables|Default|GetIsSeeingPlayer?)
    (AI|AIMoveTo self "0, 0, 0" (Game|GetPlayerCharacter 0) 1e+02 true
      (:OnSuccess
        (Variables|Default|SetCanAttack? false)
        (CallFunction|EventAttack)))))

(event Game|Damage|EventAnyDamage
  (params (Damage :type Float%20%28single-precision%29) (DamageType :type Damage%20Type%20Object%20Reference) (InstigatedBy :type Controller%20Object%20Reference) (DamageCauser :type Actor%20Object%20Reference))
  (bind _output_get (Variables|Default|SetHealth (Math|Float|Truncate (- (Variables|Default|GetHealth) Damage))))
  (if (<= _output_get 0)
    (Physics|SetSimulatePhysics (Variables|Character|GetMesh) true)))

(event Collision|EventActorBeginOverlap
  (params (OtherActor :type Actor%20Object%20Reference)))

(event EventTick
  (params (DeltaSeconds :type Float%20%28single-precision%29)))

(event EventEventAttack
  (Utilities|FlowControl|DoOnce false :!label _label
    (:Completed
      (Variables|Default|SetIsAttacking true)
      (Animation|PlayAnimMontage "/Game/EnemyZombie/Anims/Am_ZombieAttack1.Am_ZombieAttack1" 1.0 "None")
      (bind _asbp_third_person_character (Utilities|Casting|CastToBP_ThirdPersonCharacter (Game|GetPlayerCharacter 0)))
      (Game|Damage|ApplyDamage _asbp_third_person_character 1e+01 0 0 "/Script/Engine.DamageType")
      (Utilities|FlowControl|Delay 3.0)
      (Utilities|FlowControl|Sequence
        (:then_0
          (Variables|Default|SetIsAttacking false))
        (:then_1
          (goto _label Reset))))))

(fn ConstructionScript)

(fn SetTrue
  (return true))